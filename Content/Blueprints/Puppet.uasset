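; Puppet is an actor with a skeletal mesh that swaps streamed levels when the player confronts it, optionally turning its yaw toward the player on BeginPlay.
; Its See event checks an enable flag, DestroyRange and a forward-vector dot product confirming player and puppet have opposing facings.
; It then streams in NextLevel if set and, a tick later, optionally plays a pose animation before unloading CurrentLevel after a short delay.
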(event Custom|CE_Destroy
  (if (Variables|Default|Getb_Anim)
    (Components|Animation|PlayAnimation (Variables|Default|GetSkeletalMesh) "/Game/SM/Characters/Puppet/Pose/Male_Action_Pose.Male_Action_Pose" false))
  (Utilities|FlowControl|Delay 0.5)
  (Class|GameplayStatics|UnloadStreamLevelbySoftObjectPtr (Variables|Default|GetCurrentLevel) false))

(event EventBeginPlay
  (bind _asfirst_person_character (Utilities|Casting|CastToFirstPersonCharacter (Game|GetPlayerCharacter 0)))
  (Variables|Default|SetAs%20First%20Person%20Character _asfirst_person_character)
  (if (Variables|Default|Getb_StartRot)
    (Transformation|SetWorldRotation (Variables|Default|GetDefaultSceneRoot) (Math|Rotator|MakeRotator 0.0 0.0 (.yaw (Math|Rotator|FindLookatRotation (Transformation|GetActorLocation) (Transformation|GetActorLocation (Variables|Default|GetAs%20First%20Person%20Character))))) false false)))

(event EventSee
  (bind _nextlevel (Variables|Default|GetNextLevel))
  (bind _asfirst_person_character (Utilities|Casting|CastToFirstPersonCharacter (Game|GetPlayerCharacter 0)))
  (Variables|Default|SetAs%20First%20Person%20Character _asfirst_person_character)
  (if (Math|Boolean|ANDBoolean (Variables|Default|Getb_DestroyLevel) (<= (Math|Vector|Distance(Vector) (Transformation|GetActorLocation (Variables|Default|GetAs%20First%20Person%20Character)) (Transformation|GetActorLocation)) (Variables|Default|GetDestroyRange)) (< (Math|Vector|DotProduct (Transformation|GetActorForwardVector (Variables|Default|GetAs%20First%20Person%20Character)) (Transformation|GetActorForwardVector)) -0.5))
    (Utilities|FlowControl|Sequence
      (:then_0
        (if (Utilities|IsValidSoftObjectReference _nextlevel)
          (Class|GameplayStatics|LoadStreamLevelbySoftObjectPtr _nextlevel true false)))
      (:then_1
        (Utilities|FlowControl|DelayUntilNextTick)
        (CallFunction|CEDestroy)))))

(fn ConstructionScript
  (|CallParentFunction))